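; BP_BigBoss generates a maze at BeginPlay and builds it from instanced meshes.
; It centers the spawn origin along Y, then walks the grid, adding wall instances to four mesh components and storing other cells as floor transforms.
; SpawnBPClass, not called here, line-traces four sides of each floor tile and, on the first hit, adds a HISM instance offset relative to that wall, leaving persistent debug lines.
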(event `self.ReceiveBeginPlay`
  (`self.SuperGenMaze`)
  (bind _newparam (`self.Shift`))
  (`SceneComponent.K2_SetRelativeLocation` (`self.WhereToSpawn`) _newparam false false)
  (for _index (range (`self.SizeMazeX`))
    (for _index_2 (range (`self.SizeMazeZ`))
      (bind (_spawnlocation _spawnrotation _outindex) (`self.SpawnMeshComponent` _index _index_2))
      (`self.SpawnBrick` _outindex (`KismetMathLibrary.MakeTransform` _spawnlocation _spawnrotation (1.00002 1.00002 1.0)))
      (`self.shiftRoomX`))
    (`self.shiftRoomZ`))
  (`self.ClearingMemory_TEST`))

(fn `Shift`
  (returns (NewParam :type "Vector Structure"))
  (return (`KismetMathLibrary.MakeVector` 0.0 (`KismetMathLibrary.Conv_IntToDouble` (/ (* (* (`self.SizeMazeX`) (`self.SizeRoomXZ`)) -100) 2)))))

(fn `Spawn_BP_Class`
  (params (HISM_Object :type "HierarchicalInstancedStaticMeshComponent Object Reference") (PointSpawnX_or_Y :type "Float (double-precision)" :default 0.0) (PointSpawnZ :type "Float (double-precision)" :default 0.0))
  (for _array_element (`self.FloorLocation`)
    (for _array_element_2 (`self.DistanceTrace`)
      (bind _newparam (`self.Shift`))
      (bind _location (.location _array_element))
      (bind _outhit (`KismetSystemLibrary.LineTraceSingle` :`Start` (+ _location _newparam (0.0 0.0 1.0)) :`End` (+ _array_element_2 _location _newparam (0.0 0.0 1.0)) :`TraceChannel` "TraceTypeQuery1" :`DrawDebugType` "Persistent" :`bIgnoreSelf` false))
      (bind (_bblockinghit _binitialoverlap _time _location_2) (`GameplayStatics.BreakHitResult` _outhit))
      (if (!= _location_2 (0.0 0.0 0.0) :`ErrorTolerance` 0.0)
        (bind _newparam_2 (`self.Shift`))
        (bind _location_3 (.location _array_element))
        (`InstancedStaticMeshComponent.AddInstance` HISM_Object (`KismetMathLibrary.MakeTransform` (+ (* (- _location_3 (- _location_2 _newparam_2)) (`KismetMathLibrary.MakeVector` PointSpawnX_or_Y PointSpawnX_or_Y (* PointSpawnZ -1.0))) _location_3)))
        (break)))))

(fn `SpawnBrick`
  (params (IndexBrick :type Integer) (Location :type "Transform Structure"))
  (switch `int` IndexBrick
    (:`Default`
      (`KismetArrayLibrary.Array_Add` (`self.FloorLocation`) Location))
    (:`0`
      (`InstancedStaticMeshComponent.AddInstance` (`self.Wall_1`) Location))
    (:`1`
      (`InstancedStaticMeshComponent.AddInstance` (`self.Wall_2`) Location))
    (:`2`
      (`InstancedStaticMeshComponent.AddInstance` (`self.Wall_3`) Location))
    (:`3`
      (`InstancedStaticMeshComponent.AddInstance` (`self.Wall_4`) Location))))

(fn `UserConstructionScript`)