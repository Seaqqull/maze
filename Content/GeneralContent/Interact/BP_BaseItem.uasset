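; BP_BaseItem is a base interactable item that characters pick up into their inventory.
; Its construction script rebuilds the ItemInfo struct with the actor's own class, keeping the other fields as set.
; On InteractItem, it asks the instigator whether inventory space is free, then passes it ItemInfo and destroys itself.
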(event `/Game/GeneralContent/Interact/BPI_Interact.InteractItem`
  (params (Instigator :type "/Game/GeneralContent/Character/BluePrint/B_FemaleCharacter Object Reference"))
  (if (`/Game/GeneralContent/Character/BluePrint/B_FemaleCharacter.IsThereSpaceInInventory?` Instigator)
    (message `/Game/GeneralContent/Interact/BPI_Interact.PickupItem` Instigator (`self.ItemInfo`))
    (`self.K2_DestroyActor`)))

(fn `UserConstructionScript`
  (bind (_iteminfo_itemtype _iteminfo_itemname _iteminfo_itemimage _iteminfo_itemclass _iteminfo_itemindex _iteminfo_itemslot _iteminfo_itemvalue) (break `/Game/GeneralContent/Interact/S_ItemInfo` (`self.ItemInfo`)))
  (`parent.UserConstructionScript`)
  (set `self.ItemInfo` (make `/Game/GeneralContent/Interact/S_ItemInfo` _iteminfo_itemtype _iteminfo_itemname _iteminfo_itemimage (`GameplayStatics.GetObjectClass` self) _iteminfo_itemindex _iteminfo_itemslot _iteminfo_itemvalue)))