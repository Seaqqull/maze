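; Base weapon Blueprint that carries out the player character's melee-style attack and deals damage to what it hits.
; Attack runs a forward multi-sphere trace sized by WeaponInfo and the current attack's scales, then ClearHitResult prunes repeat hits on the same actor.
; Hits spawn effects, play sound and apply scaled damage, except on dead Warroks.
; Living Warroks also emit blood particles whose collisions spawn randomized splatter decals.
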(event `self.ReceiveBeginPlay`
  ;[1 1 1] CharRef
  (bind _asb_female_character (cast `/Game/GeneralContent/Character/BluePrint/B_FemaleCharacter` (`GameplayStatics.GetPlayerCharacter` 0)))
  (set `self.CharacterRef` _asb_female_character))

(event `Attack`
  (bind (_weaponinfo_type _weaponinfo_damage _weaponinfo_staminacost _weaponinfo_range _weaponinfo_horizontalwidth) (break `/Game/GeneralContent/Interact/Weapons/S_WeaponInfo` (`self.WeaponInfo`)))
  (bind (_weaponinfo_type_2 _weaponinfo_damage_2) (break `/Game/GeneralContent/Interact/Weapons/S_WeaponInfo` (`self.WeaponInfo`)))
  (bind _characterref (`self.CharacterRef`))
  (bind _characterref_2 (`self.CharacterRef`))
  (bind _returnvalue (`self.K2_GetActorLocation` _characterref_2))
  (bind ((`RangeScale_22_50C74D554CD5560A9161748D091D07CB` _rangescale) (`HorizontalWidthScale_23_64FEC6AE491B50D18D7BD186005F86C6` _horizontalwidthscale)) (break `/Game/GeneralContent/Character/BluePrint/S_Attack` (`/Game/GeneralContent/Character/BluePrint/B_FemaleCharacter.GetCurrentAttackRef` _characterref_2)))
  (bind (_outhits _returnvalue_2) (`KismetSystemLibrary.SphereTraceMulti` _returnvalue (+ _returnvalue (* (`self.GetActorForwardVector` _characterref_2) (* _weaponinfo_range _rangescale))) (* _weaponinfo_horizontalwidth _horizontalwidthscale) "TraceTypeQuery2" false (`|MakeArray` _characterref_2 :!type "Actor Object Reference")))
  (if _returnvalue_2
    (`self.ClearHitResult` _outhits)
    (for _array_element _outhits
      (bind (_bblockinghit _binitialoverlap _time _location _impactpoint _normal _impactnormal _physmat _hitactor) (`GameplayStatics.BreakHitResult` _array_element))
      (`GameplayStatics.SpawnEmitterAtLocation` null _location)
      (bind _asb_warrok_character (cast `/Game/GeneralContent/Enemy/Warrok/Blueprint/B_WarrokCharacter` _hitactor)
        (:`then`
          (if (not (`/Game/GeneralContent/Enemy/Warrok/Blueprint/BP_WarrokAnimation.IsDead?` (`/Game/GeneralContent/Enemy/Warrok/Blueprint/B_WarrokCharacter.AnimationRef` _asb_warrok_character)))
            (bind _returnvalue_3 (`GameplayStatics.SpawnEmitterAttached` "/Game/Effect/Blood/SplatterBlood_S.SplatterBlood_S" (`Character.Mesh` _asb_warrok_character) "None" (0.0 0.0 150.0)))
            (add `ParticleSystemComponent.OnParticleCollide` _returnvalue_3 (delegate `CustomEventSplittBlood`))
            (`GameplayStatics.PlaySoundAtLocation` null _location :!label _label)
            (`GameplayStatics.ApplyDamage` _hitactor (* _weaponinfo_damage_2 (`.DamageScale_19_D44894B5436021F0512CB3929F5C1AD3` (break `/Game/GeneralContent/Character/BluePrint/S_Attack` (`/Game/GeneralContent/Character/BluePrint/B_FemaleCharacter.GetCurrentAttackRef` _characterref)))) null _characterref)))
        (:`CastFailed`
          (goto _label))))))

(event `CustomEventSplittBlood`
  (params (EventName :type Name) (EmitterTime :type "Float (double-precision)") (ParticleTime :type Integer) (Location :type "Vector Structure") (Velocity :type "Vector Structure") (Direction :type "Vector Structure") (Normal :type "Vector Structure") (BoneName :type Name) (PhysMat :type "PhysicalMaterial Object Reference"))
  (bind _returnvalue (`KismetMaterialLibrary.CreateDynamicMaterialInstance` "/Game/Effect/Blood/SplatterBloodDecal_M.SplatterBloodDecal_M"))
  (`MaterialInstanceDynamic.SetScalarParameterValue` _returnvalue "Frame" (`KismetMathLibrary.Conv_IntToDouble` (`KismetMathLibrary.RandomInteger` 6)))
  (`GameplayStatics.SpawnDecalAtLocation` _returnvalue (`KismetMathLibrary.Conv_DoubleToVector` (`KismetMathLibrary.RandomFloatInRange` 5.0 10.0)) Location (`KismetMathLibrary.Conv_VectorToRotator` Normal) 20.0))

(fn `ClearHitResult`
  (params (HitArray :type "Array of HitResult Structure"))
  (for _array_element HitArray
    (for (_array_element_2 _array_index) _
      (bind (_bblockinghit _binitialoverlap _time _location _impactpoint _normal _impactnormal _physmat _hitactor) (`GameplayStatics.BreakHitResult` _array_element))
      (bind (_bblockinghit_2 _binitialoverlap_2 _time_2 _location_2 _impactpoint_2 _normal_2 _impactnormal_2 _physmat_2 _hitactor_2) (`GameplayStatics.BreakHitResult` _array_element_2))
      (if (and (!= _location _location_2) (== _hitactor _hitactor_2))
        (`KismetArrayLibrary.Array_Remove` HitArray _array_index)
        (break)))))

(fn `UserConstructionScript`
  (`parent.UserConstructionScript`))