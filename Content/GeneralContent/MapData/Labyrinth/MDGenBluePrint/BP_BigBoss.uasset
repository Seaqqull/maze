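; BP_BigBoss is a labyrinth map generator that builds the maze and its navigation area on BeginPlay.
; After SuperGenMaze, it offsets the spawn origin and loops the room grid, where SpawnBrick adds walls, floors, corners and doors as HISM instances.
; It then fits the NavMeshBoundsVolume to the maze and rebuilds navigation by console command.
; SpawnBPClass, not called here, places instances near walls found by line traces.
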(event `self.ReceiveBeginPlay`
  (bind _indexroom (`self.IndexRoom`))
  (bind _sizeroomxz (`self.SizeRoomXZ`))
  (bind _wheretospawn (`self.WhereToSpawn`))
  ;[1 1 1] Генерация и сдвиг центра лабиринта
  (`self.SuperGenMaze`)
  (bind _newparam (`self.Shift` 0 0 true)) ; Сдиг центра к игроку
  (`SceneComponent.K2_SetRelativeLocation` _wheretospawn (+ (`SceneComponent.K2_GetComponentLocation` _wheretospawn) _newparam) false false)
  (for _ (range (`self.SizeMazeX`))
    (for _ (range (`self.SizeMazeY`))
      (`self.SpawnBrick` _indexroom)
      (set `self.IndexRoom` (+ _indexroom 1))
      (`self.shiftRoomX`))
    (`self.shiftRoomZ`))
  (`self.ClearingMemory_TEST`)
  (`KismetSystemLibrary.PrintString` "Generation Completed")
  ;[1 1 1] Размещение, маштабирование зони
  (bind _newparam_2 (`self.Shift` 0 (* (`self.SizeMazeY`) 2) true true)) ; Сдиг центра к игроку
  (`self.K2_SetActorTransform` (`self.NavMeshBoundsVolume`) (`KismetMathLibrary.MakeTransform` (- (`SceneComponent.K2_GetComponentLocation` (`self.WhereToSpawn`)) _newparam_2) (struct) (`KismetMathLibrary.MakeVector` (`KismetMathLibrary.Conv_IntToDouble` (* _sizeroomxz (`self.SizeMazeY`))) (`KismetMathLibrary.Conv_IntToDouble` (* (`self.SizeMazeX`) _sizeroomxz)) 2.0)) false false)
  (`KismetSystemLibrary.Delay` 0.2)
  (`KismetSystemLibrary.ExecuteConsoleCommand` "RebuildNavigation")
  (`KismetSystemLibrary.PrintString` "RebuildNavigation Completed"))

(fn `Shift`
  (params (ErrorShiftX :type Integer) (ErrorShiftY :type Integer) (isShiftX :type Boolean) (isShiftY :type Boolean))
  (returns (NewParam :type "Vector Structure"))
  (`|ExecutionSequence`
    (:`then_0`
      (if isShiftX
        (set `self.X` (* (* (- (`self.SizeMazeX`) ErrorShiftX) (`self.SizeRoomXZ`)) 50))))
    (:`then_1`
      (if isShiftY
        (set `self.Y` (* (* (- (`self.SizeMazeY`) ErrorShiftY) (`self.SizeRoomXZ`)) 50))))
    (:`then_2`
      (return (`KismetMathLibrary.MakeVector` (`KismetMathLibrary.Conv_IntToDouble` (`self.Y`)) (`KismetMathLibrary.Conv_IntToDouble` (`self.X`)) (`KismetMathLibrary.Conv_IntToDouble` (`self.Z`)))))))

(fn `Spawn_BP_Class`
  (params (HISM_Object :type "HierarchicalInstancedStaticMeshComponent Object Reference") (PointSpawnX_or_Y :type "Float (double-precision)" :default 0.0) (PointSpawnZ :type "Float (double-precision)" :default 0.0))
  (bind _hism_floor (`self.HISM_Floor`))
  ;[1 1 1] Установка трейсов
  (for _index (range (`InstancedStaticMeshComponent.GetInstanceCount` _hism_floor))
    (for _array_element (`self.DistanceTrace`)
      (bind _location (.location (`InstancedStaticMeshComponent.GetInstanceTransform` _hism_floor _index false)))
      (bind _returnvalue (+ (`SceneComponent.K2_GetComponentLocation` (`self.WhereToSpawn`)) _location (0.0 0.0 100.0)))
      (bind _outhit (`KismetSystemLibrary.LineTraceSingle` :`Start` _returnvalue :`End` (+ _array_element _returnvalue (0.0 0.0 0.0)) :`TraceChannel` "TraceTypeQuery1" :`DrawDebugType` "Persistent" :`bIgnoreSelf` false))
      (bind (_bblockinghit _binitialoverlap _time _location_2) (`GameplayStatics.BreakHitResult` _outhit))
      ;[1 1 1] Спавн
      (if (!= _location_2 (0.0 0.0 0.0) :`ErrorTolerance` 0.0)
        (bind _returnvalue_2 (* (- (`SceneComponent.K2_GetComponentLocation` (`self.WhereToSpawn`)) _location_2) (-1.0 -1.0 1.0)))
        (`InstancedStaticMeshComponent.AddInstance` HISM_Object (`KismetMathLibrary.MakeTransform` (+ (* (- _location _returnvalue_2) (`KismetMathLibrary.MakeVector` PointSpawnX_or_Y PointSpawnX_or_Y 1.0)) _returnvalue_2 (`KismetMathLibrary.MakeVector` 0.0 0.0 PointSpawnZ))))
        (break)))))

(fn `SpawnBrick`
  (params (IndexBrick :type Integer))
  (bind _hism_corner (`self.HISM_Corner`))
  (`|ExecutionSequence`
    (:`then_0`
      (bind (_spawnlocation _spawnrotation _istrue) (`self.SpawnMeshComponent` IndexBrick))
      (if _istrue
        (`InstancedStaticMeshComponent.AddInstance` (`self.HISM_SimpleWall`) (`KismetMathLibrary.MakeTransform` _spawnlocation _spawnrotation))))
    (:`then_1`
      (bind (_spawnlocation_2 _spawnrotation_2 _istrue_2) (`self.SpawnMeshComponent` IndexBrick 1))
      (if _istrue_2
        (`InstancedStaticMeshComponent.AddInstance` (`self.HISM_SimpleWall`) (`KismetMathLibrary.MakeTransform` _spawnlocation_2 _spawnrotation_2))))
    (:`then_2`
      (bind (_spawnlocation_3 _spawnrotation_3 _istrue_3) (`self.SpawnMeshComponent` IndexBrick 2))
      (if _istrue_3
        (`InstancedStaticMeshComponent.AddInstance` (`self.HISM_SimpleWall`) (`KismetMathLibrary.MakeTransform` _spawnlocation_3 _spawnrotation_3))))
    (:`then_3`
      (bind (_spawnlocation_4 _spawnrotation_4 _istrue_4) (`self.SpawnMeshComponent` IndexBrick 3))
      (if _istrue_4
        (`InstancedStaticMeshComponent.AddInstance` (`self.HISM_SimpleWall`) (`KismetMathLibrary.MakeTransform` _spawnlocation_4 _spawnrotation_4))))
    (:`then_4`
      (bind _spawnlocation_5 (`self.SpawnMeshComponent` IndexBrick 4))
      (`InstancedStaticMeshComponent.AddInstance` (`self.HISM_Floor`) (`KismetMathLibrary.Conv_VectorToTransform` _spawnlocation_5)))
    (:`then_5`
      (bind (_spawnlocation_6 _spawnrotation_5 _istrue_5) (`self.SpawnMeshComponent` IndexBrick 5))
      (if _istrue_5
        (`InstancedStaticMeshComponent.AddInstance` _hism_corner (`KismetMathLibrary.MakeTransform` _spawnlocation_6 _spawnrotation_5))))
    (:`then_6`
      (bind (_spawnlocation_7 _spawnrotation_6 _istrue_6) (`self.SpawnMeshComponent` IndexBrick 6))
      (if _istrue_6
        (`InstancedStaticMeshComponent.AddInstance` _hism_corner (`KismetMathLibrary.MakeTransform` _spawnlocation_7 _spawnrotation_6))))
    (:`then_7`
      (bind (_spawnlocation_8 _spawnrotation_7 _istrue_7) (`self.SpawnMeshComponent` IndexBrick 7))
      (if _istrue_7
        (`InstancedStaticMeshComponent.AddInstance` (`self.HISM_Door`) (`KismetMathLibrary.MakeTransform` _spawnlocation_8 _spawnrotation_7))))))

(fn `UserConstructionScript`)