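; Preview actor that mirrors the player's equipped items on a skeletal mesh, likely for the inventory screen's character preview.
; On BeginPlay it passes itself to the player's B_FemaleCharacter, and its EquipItem and UnEquipItem events call the attach and detach functions.
; Per slot (right hand, left hand, amulet), it replaces any existing item with a spawned actor snapped to the socket named in its weapon or armor info, with collision disabled.
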(event `self.ReceiveBeginPlay`
  (bind _asb_female_character (cast `/Game/GeneralContent/Character/BluePrint/B_FemaleCharacter` (`GameplayStatics.GetPlayerCharacter` 0)))
  (`/Game/GeneralContent/Character/BluePrint/B_FemaleCharacter.PassReference` _asb_female_character self))

(event `/Game/GeneralContent/Interact/BPI_RecorderCharacter.EquipItem`
  (params (ItemInfo :type "/Game/GeneralContent/Interact/S_ItemInfo Structure"))
  (`self.AttachItem` ItemInfo))

(event `/Game/GeneralContent/Interact/BPI_RecorderCharacter.UnEquipItem`
  (params (ItemInfo :type "/Game/GeneralContent/Interact/S_ItemInfo Structure"))
  (`self.UnAttachItem` ItemInfo))

(fn `AttachItem`
  (params (ItemInfo :type "/Game/GeneralContent/Interact/S_ItemInfo Structure"))
  (bind ((`ItemClass_11_EB79B893494DE59BAC7A5D83D19F450D` _itemclass) (`ItemSlot_20_7E8B6E3A4D55772119CDC8844F163C44` _itemslot)) (break `/Game/GeneralContent/Interact/S_ItemInfo` ItemInfo))
  (bind _handrightprimaryitem (`self.HandRightPrimaryItem`))
  (bind _amuletitem (`self.AmuletItem`))
  (bind _handleftprimaryitem (`self.HandLeftPrimaryItem`))
  (switch `/Game/GeneralContent/Interact/E_SlotType` _itemslot
    (:`NewEnumerator2`
      (`/Engine/EditorBlueprintResources/StandardMacros.IsValid` _handrightprimaryitem
        (:`Is Valid`
          (`self.K2_DestroyActor` _handrightprimaryitem))
        (:`Is Not Valid`
          _))
      (bind _returnvalue (`|SpawnActorFromClass` _itemclass (`self.GetTransform`) "AlwaysSpawn" "OverrideRootScale"))
      (bind _output_get (set `self.HandRightPrimaryItem` _returnvalue))
      (bind _asbp_weapon_base (cast `/Game/GeneralContent/Interact/Weapons/BP_WeaponBase` _output_get))
      (`self.K2_AttachToComponent` _asbp_weapon_base (`self.SkeletalMesh`) (`.PrimaryRightHand_50_2B3F65E04C46F161DCF873967F90BE3A` (break `/Game/GeneralContent/Interact/Weapons/S_WeaponInfo` (`/Game/GeneralContent/Interact/Weapons/BP_WeaponBase.WeaponInfo` _asbp_weapon_base))) "SnapToTarget" "SnapToTarget" "SnapToTarget" true)
      (`self.SetActorEnableCollision` _asbp_weapon_base false))
    (:`NewEnumerator3`
      (`/Engine/EditorBlueprintResources/StandardMacros.IsValid` _handleftprimaryitem
        (:`Is Valid`
          (`self.K2_DestroyActor` _handleftprimaryitem))
        (:`Is Not Valid`
          _))
      (bind _returnvalue_2 (`|SpawnActorFromClass` _itemclass (`self.GetTransform`) "AlwaysSpawn" "OverrideRootScale"))
      (bind _output_get_2 (set `self.HandLeftPrimaryItem` _returnvalue_2))
      (bind _asbp_weapon_base_2 (cast `/Game/GeneralContent/Interact/Weapons/BP_WeaponBase` _output_get_2))
      (`self.K2_AttachToComponent` _asbp_weapon_base_2 (`self.SkeletalMesh`) (`.PrimaryLeftHand_51_551AB3254CD8BB8A27F659BE62C7E3B4` (break `/Game/GeneralContent/Interact/Weapons/S_WeaponInfo` (`/Game/GeneralContent/Interact/Weapons/BP_WeaponBase.WeaponInfo` _asbp_weapon_base_2))) "SnapToTarget" "SnapToTarget" "SnapToTarget" true)
      (`self.SetActorEnableCollision` _asbp_weapon_base_2 false))
    (:`NewEnumerator6`
      (`/Engine/EditorBlueprintResources/StandardMacros.IsValid` _amuletitem
        (:`Is Valid`
          (`self.K2_DestroyActor` _amuletitem))
        (:`Is Not Valid`
          _))
      (bind _returnvalue_3 (`|SpawnActorFromClass` _itemclass (`self.GetTransform`) "AlwaysSpawn" "OverrideRootScale"))
      (bind _output_get_3 (set `self.AmuletItem` _returnvalue_3))
      (bind _asbp_armor_base (cast `/Game/GeneralContent/Interact/Armor/BP_ArmorBase` _output_get_3))
      (`self.K2_AttachToComponent` _asbp_armor_base (`self.SkeletalMesh`) (`.AttachPoint_15_B5932E1A4452F50C5E64118CB06D1B68` (break `/Game/GeneralContent/Interact/Armor/S_ArmorInfo` (`/Game/GeneralContent/Interact/Armor/BP_ArmorBase.ArmorInfo` _asbp_armor_base))) "SnapToTarget" "SnapToTarget" "SnapToTarget" true)
      (`self.SetActorEnableCollision` _asbp_armor_base false))))

(fn `UnAttachItem`
  (params (ItemInfo :type "/Game/GeneralContent/Interact/S_ItemInfo Structure"))
  (switch `/Game/GeneralContent/Interact/E_SlotType` (`.ItemSlot_20_7E8B6E3A4D55772119CDC8844F163C44` (break `/Game/GeneralContent/Interact/S_ItemInfo` ItemInfo))
    (:`NewEnumerator2`
      (`self.K2_DestroyActor` (`self.HandRightPrimaryItem`)))
    (:`NewEnumerator3`
      (`self.K2_DestroyActor` (`self.HandLeftPrimaryItem`)))
    (:`NewEnumerator6`
      (`self.K2_DestroyActor` (`self.AmuletItem`)))))

(fn `UserConstructionScript`)